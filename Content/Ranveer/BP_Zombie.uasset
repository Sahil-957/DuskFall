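; Zombie AI pawn that wanders at random and chases any pawn it sees.
; Roaming walks slowly to random reachable points within a large radius, pausing briefly after each successful move before picking the next.
; PawnSensing sightings raise the speed and start a move toward the seen pawn.
; Each sighting also resets a short retriggerable delay, so roaming resumes shortly after sightings stop.
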(event OnSeePawn(PawnSensing)
  (params (Pawn :type Pawn%20Object%20Reference))
  (Utilities|FlowControl|Sequence
    (:then_0
      (Variables|/Script/Engine.CharacterMovementComponent|SetMaxWalkSpeed (Variables|Character|GetCharacterMovement) 5e+02)
      (AI|AIMoveTo self "0, 0, 0" Pawn 2e+02 false))
    (:then_1
      (Utilities|FlowControl|RetriggerableDelay 0.2)
      (CallFunction|Roaming))))

(event Custom|Roaming
  (Variables|/Script/Engine.CharacterMovementComponent|SetMaxWalkSpeed (Variables|Character|GetCharacterMovement) 1.5e+02)
  (AI|AIMoveTo self (.RandomLocation (AI|Navigation|GetRandomReachablePointinRadius (Transformation|GetWorldLocation (Variables|Character|GetMesh)) 8e+03 0 0)) 0 5.0 false
    (:OnSuccess
      (Utilities|FlowControl|Delay (Math|Random|RandomFloatinRange 0.0 4.0))
      (CallFunction|Roaming))))

(event EventBeginPlay
  (CallFunction|Roaming))

(fn ConstructionScript)